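; Player-controlled tank Blueprint that wires up its turret, barrel, camera aiming and fire input.
; On BeginPlay it passes the Turret and TankBarrel components to setter functions defined outside these graphs.
; Horizontal aim input yaws a gimbal and vertical input pitches the spring arm, both by raw axis value without delta-time scaling.
; The Fire action calls a Fire function, also defined elsewhere.
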(event `self.ReceiveBeginPlay`
  (`self.SetTurretReference` (`self.Turret`))
  (`self.SetBarrelReference` (`self.Tank Barrel`)))

(event `InputAxis|AimHorizontal`
  (params (AxisValue :type "Float (single-precision)"))
  ;[1 1 1] Controls
  (`SceneComponent.K2_AddLocalRotation` (`self.HorizontalGimbal`) (`KismetMathLibrary.MakeRotator` 0.0 0.0 AxisValue) false false))

(event `InputAction|Fire`
  (params (Key :type "Key Structure"))
  ;[1 1 1] Controls
  (:`Pressed`
    (`self.Fire`)))

(event `InputAxis|AimVertical`
  (params (AxisValue :type "Float (single-precision)"))
  ;[1 1 1] Controls
  (`SceneComponent.K2_AddLocalRotation` (`self.SpringArm`) (`KismetMathLibrary.MakeRotator` 0.0 AxisValue) false false))

(fn `UserConstructionScript`)